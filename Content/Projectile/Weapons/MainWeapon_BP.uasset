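; Base-style main weapon actor for a character, providing automatic hitscan fire with ammo and timed reload, despite its Projectile folder.
; Input events call server-style SR events; a looping timer drives shots, with negative start delay for an immediate first round.
; Each allowed shot spends ammo and line-traces from the character's ProjectileSpawnPoint to apply damage.
; MC multicast-style events play sounds and spawn Niagara muzzle and impact effects.
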(event `/Game/TopDown/Blueprints/Interfaces/Tools_BPI.Setup_Actor`
  (params (Character :type "/Game/TopDown/Blueprints/GameModes/Core/Core_Character_BP Object Reference"))
  (set `self.Char_Ref` Character))

(event `/Game/Projectile/Inputs_BPI.Input_PrimaryActionPressed`
  ; Inputs
  (`self.SR_PrimaryAction` true))

(event `/Game/Projectile/Inputs_BPI.Input_PrimaryActionReleased`
  ; Inputs
  (`self.SR_PrimaryAction` false))

(event `/Game/Projectile/Inputs_BPI.Input_Reload`
  ; Reload
  (`self.SR_Reload`))

(event `SR_Reload`
  ; Reload
  (`self.CanReload?`
    (:`true`
      (set `self.Reloading?` true)
      (`self.MC_Reload`)
      (`KismetSystemLibrary.Delay` (`self.ReloadDuration`))
      (set `self.Ammo` (`self.MaxAmmo`))
      (set `self.Reloading?` false))))

(event `MC_Reload`
  ; Reload
  (`GameplayStatics.SpawnSoundAttached` (`self.ReloadSoundEffect`) (`self.StaticMesh`) "None" (0.0 0.0 0.0) (struct) "KeepRelativeOffset" false 1.0 1.0 0.0 null null))

(event `SR_PrimaryAction`
  (params (`Pressed?` :type Boolean))
  (bind _rateoffire (`self.RateOfFire`))
  ; Shooting
  (if `Pressed?`
    (bind _returnvalue (`KismetSystemLibrary.K2_SetTimerDelegate` (delegate `Shooting`) _rateoffire true false (* _rateoffire -1.0)))
    (set `self.TH_Shooting` _returnvalue)
    (else
      (`KismetSystemLibrary.K2_ClearAndInvalidateTimerHandle` (`self.TH_Shooting`)))))

(event `Shooting`
  ; Shooting
  (`self.CanShoot?`
    (:`true`
      (`/Engine/EditorBlueprintResources/StandardMacros.DecrementInt` (`self.Ammo`)
        (:`  `
          (`self.MC_Shoot`)
          (`self.MC_SpawnMuzzleFlash` (0.0 0.0 0.0))
          (`self.LineTrace_Shot`))))))

(event `MC_Shoot`
  ; Shooting
  (`GameplayStatics.SpawnSoundAttached` (`self.ShootingSoundEffect`) (`self.StaticMesh`) "None" (0.0 0.0 0.0) (struct) "KeepRelativeOffset" false 1.0 1.0 0.0 null null))

(event `MC_SpawnMuzzleFlash`
  (params (Normal :type "Vector Structure"))
  ; Shooting
  (`NiagaraFunctionLibrary.SpawnSystemAtLocation` "/Game/Projectile/vfx/MuzzleFlash/NS_MuzzleFlash.NS_MuzzleFlash" (`SceneComponent.GetSocketLocation` (`/Game/TopDown/Blueprints/GameModes/Core/Core_Character_BP.ProjectileSpawnPoint` (`self.Char_Ref`)) "None") (`KismetMathLibrary.Conv_VectorToRotator` Normal) (3.0 3.0 3.0)))

(event `MC_SpawnImpact`
  (params (Location :type "Vector Structure") (Normal :type "Vector Structure"))
  ; Shooting
  (`NiagaraFunctionLibrary.SpawnSystemAtLocation` "/Game/MixedVFX/Particles/Explosions/NS_ExplosionMidAirSmall.NS_ExplosionMidAirSmall" Location (`KismetMathLibrary.Conv_VectorToRotator` Normal)))

(fn `LineTrace_Shot`
  (bind _projectilespawnpoint (`/Game/TopDown/Blueprints/GameModes/Core/Core_Character_BP.ProjectileSpawnPoint` (`self.Char_Ref`)))
  (bind _returnvalue (`SceneComponent.K2_GetComponentLocation` _projectilespawnpoint))
  (bind _returnvalue_2 (`SceneComponent.GetForwardVector` _projectilespawnpoint))
  (bind (_outhit _returnvalue_3) (`KismetSystemLibrary.LineTraceSingle` (+ _returnvalue _returnvalue_2) (+ _returnvalue (* _returnvalue_2 (`self.ShootingRange`))) "TraceTypeQuery1" false (`|MakeArray` (`self.Char_Ref`) :!type "Actor Object Reference")))
  (if _returnvalue_3
    (bind (_bblockinghit _binitialoverlap _time _distance _location _impactpoint _normal _impactnormal _physmat _hitactor) (`GameplayStatics.BreakHitResult` _outhit))
    (`self.MC_SpawnImpact` _location _normal)
    (`GameplayStatics.ApplyDamage` _hitactor (`self.Damage`) (`self.GetInstigatorController` (`self.Char_Ref`)) self)))

(fn `UserConstructionScript`
  (`StaticMeshComponent.SetStaticMesh` (`self.StaticMesh`) (`self.Weapon_Mesh`)))