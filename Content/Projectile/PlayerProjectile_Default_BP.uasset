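; Default player projectile actor that damages enemies on impact.
; On Hit it checks the other actor for the Enemy tag, applies fixed damage with a debug print, and destroys itself whatever it struck.
; The PickUp event is empty, and leftover weapon-equip, socket-attach and Niagara fairy-arrow nodes are disconnected and never run.
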(event `self.ReceiveBeginPlay`)

(event `/Game/Projectile/InterWithWeapons.PickUp`
  ; PickUp
)

(event `self.ReceiveHit`
  (params (MyComp :type "PrimitiveComponent Object Reference") (Other :type "Actor Object Reference") (OtherComp :type "PrimitiveComponent Object Reference") (bSelfMoved :type Boolean) (HitLocation :type "Vector Structure") (HitNormal :type "Vector Structure") (NormalImpulse :type "Vector Structure") (Hit :type "HitResult Structure (by ref)"))
  ; Damage Enemy
  (if (`self.ActorHasTag` Other "Enemy")
    (`GameplayStatics.ApplyDamage` Other 25.0)
    (`KismetSystemLibrary.PrintString` "Bullet fired" true true (struct :`R` 1.0 :`G` 0.942168 :`A` 1.0))
    (`self.K2_DestroyActor`)
    (else
      (`self.K2_DestroyActor`))))

(fn `UserConstructionScript`)