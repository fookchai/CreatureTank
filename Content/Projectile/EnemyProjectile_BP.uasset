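; Enemy projectile actor that damages the player on impact.
; On BeginPlay it assigns the galaxy arrow Niagara effect, provided the player pawn casts to ET-01_BP.
; The Hit event applies fixed damage to actors tagged Player and prints a debug string, and the projectile destroys itself on any hit.
; The Sphere overlap event is empty.
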(event `self.ReceiveBeginPlay`
  (cast `/Game/Characters/Enemy/ET-01/Blueprint/ET-01_BP` (`GameplayStatics.GetPlayerPawn` 0))
  (`NiagaraComponent.SetAsset` (`self.Niagara`) "/Game/MixedVFX/Particles/Projectiles/NS_GalaxyArrow.NS_GalaxyArrow" true))

(event `self.Sphere.OnComponentBeginOverlap`
  (params (OverlappedComponent :type "PrimitiveComponent Object Reference") (OtherActor :type "Actor Object Reference") (OtherComp :type "PrimitiveComponent Object Reference") (OtherBodyIndex :type Integer) (bFromSweep :type Boolean) (SweepResult :type "HitResult Structure (by ref)")))

(event `self.ReceiveHit`
  (params (MyComp :type "PrimitiveComponent Object Reference") (Other :type "Actor Object Reference") (OtherComp :type "PrimitiveComponent Object Reference") (bSelfMoved :type Boolean) (HitLocation :type "Vector Structure") (HitNormal :type "Vector Structure") (NormalImpulse :type "Vector Structure") (Hit :type "HitResult Structure (by ref)"))
  (if (`self.ActorHasTag` Other "Player")
    (`GameplayStatics.ApplyDamage` Other 5.0)
    (`KismetSystemLibrary.PrintString` "Bullet fired")
    (`self.K2_DestroyActor`)
    (else
      (`self.K2_DestroyActor`))))

(fn `UserConstructionScript`)