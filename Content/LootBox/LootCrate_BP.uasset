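; Interactable loot crate that opens once and spawns one to three random pickups inside its spawning volume.
; Interact sets Opened and spawns items, picking random DT_PickupItems rows and rerolling until one passes its SpawnPercentage.
; The Opened OnRep plays the lid timeline; a separate cosmetic event, uncalled here, plays a sound.
; Focus shows the "Lootbox" prompt widget, hidden by a retriggerable delay once focus calls stop.
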(event `self.ReceiveBeginPlay`
  (`self.Setup InteractionWidget`))

(event `SpawnItems`
  (bind _output_get (set `self.LootSpawnAmount` (`KismetMathLibrary.RandomIntegerInRange` 1 3)))
  (bind _counter (`/Engine/EditorBlueprintResources/StandardMacros.Do N` _output_get :!label _label)
    (:`Exit`
      (`self.SpawnActualItem`)
      (if (not (== _counter (`self.LootSpawnAmount`)))
        (goto _label)))))

(event `SpawnActualItem`
  (bind _outrownames (`DataTableFunctionLibrary.GetDataTableRowNames` "/Game/Data/DT_PickupItems.DT_PickupItems" :!label _label_2))
  (bind _returnvalue (`|GetDataTableRow` "/Game/Data/DT_PickupItems.DT_PickupItems" (`KismetArrayLibrary.Array_Random` _outrownames))
    (:`then`
      (bind (_id _name _sm_item _spawnpercentage) (break `/Game/Data/S_PickupItem` _returnvalue))
      (if (<= (`KismetMathLibrary.RandomFloatInRange` 0.0 100.0) _spawnpercentage)
        (`|SpawnActorFromClass` "/Game/Projectile/PickUp_Items_BP.PickUp_Items_BP_C" (`KismetMathLibrary.MakeTransform` (`KismetMathLibrary.RandomPointInBoundingBox` (`SceneComponent.K2_GetComponentLocation` (`self.SpawningVolume`)) (`BoxComponent.GetUnscaledBoxExtent` (`self.SpawningVolume`)))) "AdjustIfPossibleButAlwaysSpawn" "MultiplyWithRoot" null _id null)
        (else
          (goto _label_2))))))

(event `/Game/TopDown/Blueprints/Interfaces/Interaction_BPI.Interact`
  (params (interactingActor :type "Actor Object Reference"))
  (if (not (`self.Opened?`))
    (set `self.Opened?` true)
    (`self.SpawnItems`)))

(event `/Game/TopDown/Blueprints/Interfaces/Interaction_BPI.SetFocused`
  (`SceneComponent.SetVisibility` (`self.Widget`) true false)
  (`KismetSystemLibrary.RetriggerableDelay` 0.1)
  (`SceneComponent.SetVisibility` (`self.Widget`) false false))

(event `openCrate`
  ; Open Lid Event
  (bind (_direction _lidrotation) (`Timeline|CrateOpening_TL` :!via `PlayFromStart`)
    (:`Update`
      (`SceneComponent.K2_SetRelativeRotation` (`self.Scene`) (`KismetMathLibrary.MakeRotator` _lidrotation) false false))))

(event `MC_CosmeticOpening`
  ; Cosmetic Event
  (`GameplayStatics.PlaySoundAtLocation` null (`self.K2_GetActorLocation`) (struct) 1.0 1.0 0.0 null null null null))

(fn `OnRep_Opened?`
  (`self.openCrate`))

(fn `Setup InteractionWidget`
  (bind _asinteraction_feed_back_wb (cast `/Game/Widget/InteractionFeedBack_WB` (`WidgetComponent.GetWidget` (`self.Widget`))))
  (`/Game/Widget/InteractionFeedBack_WB.Update Widget` _asinteraction_feed_back_wb "Lootbox"))

(fn `UserConstructionScript`)