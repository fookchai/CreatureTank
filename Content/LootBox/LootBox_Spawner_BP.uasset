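; Loot box spawner actor that scatters a random number of loot crates across the area of its Box when play begins, then destroys itself.
; A DoN loop calls SpawnLoot 5 to 20 times.
; Each call line-traces on Visibility from a random point in the box down to a fixed low world Z.
; On a hit, it spawns a LootCrate_BP there, rotated from the surface normal.
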(event `self.ReceiveBeginPlay`
  (set `self.AmountOfLoot` (`KismetMathLibrary.RandomIntegerInRange` 5 20))
  (bind _counter (`/Engine/EditorBlueprintResources/StandardMacros.Do N` (`self.AmountOfLoot`) :!label _label)
    (:`Exit`
      (`self.SpawnLoot`)
      (if (== _counter (`self.AmountOfLoot`))
        (`self.K2_DestroyActor`)
        (else
          (goto _label))))))

(fn `SpawnLoot`
  (bind _returnvalue (`KismetMathLibrary.RandomPointInBoundingBox` (`SceneComponent.K2_GetComponentLocation` (`self.Box`)) (`BoxComponent.GetUnscaledBoxExtent` (`self.Box`))))
  (bind (_outhit _returnvalue_2) (`KismetSystemLibrary.LineTraceSingle` _returnvalue (`KismetMathLibrary.MakeVector` (.x _returnvalue) (.y _returnvalue) -2000.0) "TraceTypeQuery1"))
  (if _returnvalue_2
    (bind (_bblockinghit _binitialoverlap _time _distance _location _impactpoint _normal) (`GameplayStatics.BreakHitResult` _outhit))
    (`|SpawnActorFromClass` "/Game/LootBox/LootCrate_BP.LootCrate_BP_C" (`KismetMathLibrary.MakeTransform` _location (`KismetMathLibrary.MakeRotator` (.roll (`KismetMathLibrary.Conv_VectorToRotator` _normal)) (- (.pitch (`KismetMathLibrary.Conv_VectorToRotator` _normal)) 90.0) (- (.yaw (`KismetMathLibrary.Conv_VectorToRotator` _normal)) -90.0))) "Undefined" "MultiplyWithRoot" null null)))

(fn `UserConstructionScript`)