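; Health component that tracks the health of its owning actor as it takes damage.
; On BeginPlay it fills Health to MaxHealth and binds to the owner's OnTakeAnyDamage event.
; Each hit subtracts damage, clamps the result between zero and MaxHealth, and broadcasts OnHealthChange with the new value.
; It also broadcasts OnHealthDepletetd whenever a hit leaves Health at zero, with no guard against repeat calls.
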(event `self.ReceiveBeginPlay`
  ; Damage Player
  (set `self.Health` (`self.MaxHealth`))
  (add `Actor.OnTakeAnyDamage` (`self.GetOwner`) (delegate `OnDamgeTaken`)))

(event `OnDamgeTaken`
  (params (DamagedActor :type "Actor Object Reference") (Damage :type "Float (single-precision)") (DamageType :type "DamageType Object Reference") (InstigatedBy :type "Controller Object Reference") (DamageCauser :type "Actor Object Reference"))
  ; Damage Player
  (bind _output_get (set `self.Health` (`KismetMathLibrary.FClamp` (- (`self.Health`) Damage) 0.0 (`self.MaxHealth`))))
  (`self.OnHealthChange` _output_get)
  (if (<= (`self.Health`) 0.0)
    (`self.OnHealthDepletetd`)))