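; ET-01 enemy character that chases seen characters and fires projectiles at them.
; Pawn sensing starts an AI move toward the target and a delayed projectile spawn, while a retriggerable delay clears sight and toggles the anim blueprint's Deactivate flag.
; When sight is lost, Tick issues delayed AI moves without a target.
; Health component events play damage or defeat animations, print debug text, and remove sensing on death.
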(event `self.ReceiveTick`
  (params (DeltaSeconds :type "Float (single-precision)"))
  ; Chase Player
  (if (not (`self.Can See player?`))
    (`KismetSystemLibrary.Delay` 0.2)
    (`|AIMoveTo` self (0.0 0.0 0.0) null 20.0 true)))

(event `self.PawnSensing.OnSeePawn`
  (params (Pawn :type "Pawn Object Reference"))
  (bind _aset_01_abp (cast `/Game/Characters/Enemy/ET-01/Blueprint/ET-01_ABP` (`SkeletalMeshComponent.GetAnimInstance` (`self.Mesh`)) :!pure true))
  ; Chase Player
  (bind _ascharacter (cast `Character` Pawn))
  (`|ExecutionSequence`
    (:`then_0`
      (set `self.Can See player?` true)
      (set `/Game/Characters/Enemy/ET-01/Blueprint/ET-01_ABP.Deactivate?` false _aset_01_abp)
      (`|AIMoveTo` self (0.0 0.0 0.0) _ascharacter 5.0 true
        (:`then`
          (`KismetSystemLibrary.Delay` 2.0)
          ; Attack Player
          (`|SpawnActorFromClass` "/Game/Projectile/EnemyProjectile_BP.EnemyProjectile_BP_C" (`SceneComponent.K2_GetComponentToWorld` (`self.ProjectileSpawnPoint`)) "AdjustIfPossibleButAlwaysSpawn" "MultiplyWithRoot" null null)
          (`SkeletalMeshComponent.PlayAnimation` (`self.Mesh`) "/Game/Characters/Enemy/ET-01/Animations/Fire.Fire" false))))
    (:`then_1`
      (`KismetSystemLibrary.RetriggerableDelay` 0.6)
      (set `self.Can See player?` false)
      (set `/Game/Characters/Enemy/ET-01/Blueprint/ET-01_ABP.Deactivate?` true _aset_01_abp))))

(event `Is Dead`)

(event `self.HealthComponent_BP.OnHealthChange`
  (params (NewHealth :type "Float (double-precision)"))
  ; Health Component
  (`SkeletalMeshComponent.PlayAnimation` (`self.Mesh`) "/Game/Characters/Enemy/ET-01/Animations/Damage.Damage" false)
  (`KismetSystemLibrary.PrintString` (`KismetStringLibrary.Concat_StrStr` "NewHealth:" (`KismetStringLibrary.Conv_DoubleToString` NewHealth)) true true (struct :`R` 0.017513 :`G` 0.51875 :`A` 1.0) 2.0 "Health"))

(event `self.HealthComponent_BP.OnHealthDepletetd`
  ; Health Component
  (`KismetSystemLibrary.PrintString` "Enemy Die" true true (struct :`R` 0.689583 :`B` 0.046434 :`A` 1.0))
  (`SkeletalMeshComponent.PlayAnimation` (`self.Mesh`) "/Game/Characters/Enemy/ET-01/Animations/Defeated.Defeated" false)
  (`ActorComponent.K2_DestroyComponent` (`self.PawnSensing`)))

(fn `UserConstructionScript`)