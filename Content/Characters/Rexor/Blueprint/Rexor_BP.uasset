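; Player-controlled Rexor character with tank-style body driving, an independently turning head and swappable weapons.
; Tick averages GroundSencing_BP hits to align the body to terrain height and slope, and traces for interactables.
; Turret input drives the AnimBP head angle, returning to idle after a delay.
; A two-slot RepNotify inventory uses DT_PickupItems to set the active weapon child actor and spare-slot mesh; fire and reload are forwarded to that weapon.
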(event `self.ReceiveBeginPlay`
  ;[0.05098 0.05098 0.05098] Add Mapping Context
  (bind _asplayer_controller (cast `PlayerController` (`self.GetController`)))
  (bind _returnvalue (pcsubsystem `EnhancedInputLocalPlayerSubsystem` _asplayer_controller))
  (`/Engine/EditorBlueprintResources/StandardMacros.IsValid` _returnvalue
    (:`Is Valid`
      (`EnhancedInputSubsystemInterface.AddMappingContext` _returnvalue "/Game/TopDown/Input/IMC_Default.IMC_Default" 0 (struct))
      (set `self.GroundSensingArray` (`self.K2_GetComponentsByClass` "/Game/TopDown/Blueprints/GroundSencing_BP.GroundSencing_BP_C"))
      (set `PlayerController.bShowMouseCursor` true (`GameplayStatics.GetPlayerController` 0))
      (bind _asrexor_skeleton_anim_blueprint (cast `/Game/Characters/Rexor/Blueprint/Rexor_Skeleton_AnimBlueprint` (`SkeletalMeshComponent.GetAnimInstance` (`self.Mesh`))))
      (set `self.Is_Idle?` (`/Game/Characters/Rexor/Blueprint/Rexor_Skeleton_AnimBlueprint.Is Idle?` _asrexor_skeleton_anim_blueprint))
      (set `self.Ref to AnimeBP` _asrexor_skeleton_anim_blueprint))))

(event `EnhancedInput|/Game/TopDown/Input/Actions/IA_Interact`
  (params (ActionValue :type Boolean) (ElapsedSeconds :type "Float (double-precision)") (TriggeredSeconds :type "Float (double-precision)") (InputAction :type "InputAction Object Reference" :default "/Game/TopDown/Input/Actions/IA_Interact.IA_Interact"))
  (:`Triggered`
    (message `/Game/TopDown/Blueprints/Interfaces/Interaction_BPI.Interact` (`self.InteractionActor`) self)))

(event `EnhancedInput|/Game/TopDown/Input/Actions/IA_BodyDrive`
  (params (ActionValue :type "Float (double-precision)") (ElapsedSeconds :type "Float (double-precision)") (TriggeredSeconds :type "Float (double-precision)") (InputAction :type "InputAction Object Reference" :default "/Game/TopDown/Input/Actions/IA_BodyDrive.IA_BodyDrive"))
  ; Body move Forward/Backward
  (:`Triggered`
    (set `self.TargetForwardSpeed` (* ActionValue (`self.MaxForwardSpeed`))))
  (:`Completed`
    (set `self.TargetForwardSpeed` 0.0)))

(event `EnhancedInput|/Game/TopDown/Input/Actions/IA_BodyTurn`
  (params (ActionValue :type "Float (double-precision)") (ElapsedSeconds :type "Float (double-precision)") (TriggeredSeconds :type "Float (double-precision)") (InputAction :type "InputAction Object Reference" :default "/Game/TopDown/Input/Actions/IA_BodyTurn.IA_BodyTurn"))
  ; Body turn
  (:`Triggered`
    (set `self.TargetTurnSpeed` (* ActionValue (`self.MaxTurnSpeed`))))
  (:`Completed`
    (set `self.TargetTurnSpeed` 0.0)))

(event `Start Idle`
  ; Head/Turret Turn
  (set `/Game/Characters/Rexor/Blueprint/Rexor_Skeleton_AnimBlueprint.Is Idle?` true (cast `/Game/Characters/Rexor/Blueprint/Rexor_Skeleton_AnimBlueprint` (`SkeletalMeshComponent.GetAnimInstance` (`self.Mesh`)) :!pure true)))

(event `EnhancedInput|/Game/TopDown/Input/Actions/IA_Turret`
  (params (ActionValue :type "Float (double-precision)") (ElapsedSeconds :type "Float (double-precision)") (TriggeredSeconds :type "Float (double-precision)") (InputAction :type "InputAction Object Reference" :default "/Game/TopDown/Input/Actions/IA_Turret.IA_Turret"))
  (bind _returnvalue (`GameplayStatics.GetWorldDeltaSeconds`))
  (bind _currentmouthangle (`self.CurrentMouthAngle`))
  (bind _currentheadangle (`self.CurrentHeadAngle`))
  (bind _ref_to_animebp (`self.Ref to AnimeBP`))
  ; Head/Turret Turn
  (:`Triggered`
    (bind _output_get (set `self.CurrentHeadAngle` (mod (`KismetMathLibrary.FInterpTo` _currentheadangle (+ _currentheadangle (* (`self.HeadRotationSpeed`) (`KismetMathLibrary.BreakVector2D` (`KismetMathLibrary.Conv_DoubleToVector2D` ActionValue)) _returnvalue)) _returnvalue 25.0) 360.0)))
    (set `/Game/Characters/Rexor/Blueprint/Rexor_Skeleton_AnimBlueprint.HeadAngle` _output_get _ref_to_animebp)
    (bind _output_get_2 (set `self.CurrentMouthAngle` (`KismetMathLibrary.ClampAngle` (`KismetMathLibrary.FInterpTo` _currentmouthangle (+ _currentmouthangle (* 0.0 _returnvalue (`self.MouthRotSpeed`))) _returnvalue 25.0) -35.0 10.0)))
    (set `/Game/Characters/Rexor/Blueprint/Rexor_Skeleton_AnimBlueprint.MouthAngle` _output_get_2 _ref_to_animebp)
    (set `/Game/Characters/Rexor/Blueprint/Rexor_Skeleton_AnimBlueprint.Is Idle?` false (cast `/Game/Characters/Rexor/Blueprint/Rexor_Skeleton_AnimBlueprint` (`SkeletalMeshComponent.GetAnimInstance` (`self.Mesh`)) :!pure true))
    (`KismetSystemLibrary.K2_ClearAndInvalidateTimerHandle` (stale _returnvalue_2)))
  (:`Completed`
    (bind _returnvalue_2 (`KismetSystemLibrary.K2_SetTimerDelegate` (delegate `Start Idle`) 5.0))))

(event `EnhancedInput|/Game/TopDown/Input/Actions/IA_Fire`
  (params (ActionValue :type Boolean) (ElapsedSeconds :type "Float (double-precision)") (TriggeredSeconds :type "Float (double-precision)") (InputAction :type "InputAction Object Reference" :default "/Game/TopDown/Input/Actions/IA_Fire.IA_Fire"))
  (bind _childactor (`ChildActorComponent.ChildActor` (`self.ActiveWeapon`)))
  ; Shooting
  (:`Triggered`
    (if ActionValue
      (`/Engine/EditorBlueprintResources/StandardMacros.IsValid` _childactor
        (:`Is Valid`
          (message `/Game/Projectile/Inputs_BPI.Input_PrimaryActionPressed` _childactor)))
      (else
        (`/Engine/EditorBlueprintResources/StandardMacros.IsValid` _childactor
          (:`Is Valid`
            (message `/Game/Projectile/Inputs_BPI.Input_PrimaryActionReleased` _childactor)))))))

(event `self.ReceiveTick`
  (params (DeltaSeconds :type "Float (single-precision)"))
  (bind (_returnvalue_x _returnvalue_y _returnvalue_z) (`KismetMathLibrary.BreakVector` (`self.K2_GetActorLocation`)))
  (bind _returnvalue (`GameplayStatics.GetWorldDeltaSeconds`))
  (bind _returnvalue_2 (`GameplayStatics.GetWorldDeltaSeconds`))
  (bind _returnvalue_3 (`KismetMathLibrary.FInterpTo` (`self.CurrentForwardSpeed`) (`self.TargetForwardSpeed`) _returnvalue 2.0))
  ; Ground Sensing
  (set `self.AverageNormal` (0.0 0.0 0.0))
  (set `self.AverageHeight` 0.0)
  (set `self.CountOnGround` 0)
  (for _array_element (`self.GroundSensingArray`)
    (set `self.AverageNormal` (+ (`/Game/TopDown/Blueprints/GroundSencing_BP.HitNormal` _array_element) (`self.AverageNormal`)))
    (bind (_hitlocation_x _hitlocation_y _hitlocation_z) (`KismetMathLibrary.BreakVector` (`/Game/TopDown/Blueprints/GroundSencing_BP.HitLocation` _array_element)))
    (set `self.AverageHeight` (+ _hitlocation_z (`self.AverageHeight`)))
    (if (`/Game/TopDown/Blueprints/GroundSencing_BP.bOnGround` _array_element)
      (`/Engine/EditorBlueprintResources/StandardMacros.IncrementInt` (`self.CountOnGround`)
        (:`  `
          (`self.InteractionTrace`)))))
  (set `self.AverageNormal` (/ (`self.AverageNormal`) (`self.CountOnGround`)))
  (bind _output_get (set `self.AverageHeight` (/ (`self.AverageHeight`) (`self.CountOnGround`))))
  (set `self.DeltaZ` (- (+ _output_get (`self.HeightOffset`)) _returnvalue_z))
  (`self.K2_SetActorRotation` (`KismetMathLibrary.RInterpTo` (`self.K2_GetActorRotation`) (`KismetMathLibrary.ComposeRotators` (`KismetMathLibrary.MakeRotator` 0.0 0.0 (* (`self.TargetTurnSpeed`) _returnvalue_2)) (`KismetMathLibrary.MakeRotFromZY` (`self.AverageNormal`) (`self.GetActorRightVector`))) _returnvalue_2 8.0))
  (`self.K2_AddActorWorldOffset` (+ (* (`self.GetActorForwardVector`) _returnvalue_3 _returnvalue) (* (`self.GetActorUpVector`) (`self.DeltaZ`))))
  (set `self.CurrentForwardSpeed` _returnvalue_3))

(event `/Game/TopDown/Blueprints/Interfaces/Tools_BPI.Handle_Pickup`
  (params (ID :type String))
  ; Pickup item check
  (`self.Process_ItemPickup` ID)
  (`GameplayStatics.PlaySound2D` (`self.PickupSoundEffect`) 1.0 1.0 0.0 null null))

(event `EnhancedInput|/Game/TopDown/Input/Actions/IA_Slot1`
  (params (ActionValue :type Boolean) (ElapsedSeconds :type "Float (double-precision)") (TriggeredSeconds :type "Float (double-precision)") (InputAction :type "InputAction Object Reference" :default "/Game/TopDown/Input/Actions/IA_Slot1.IA_Slot1"))
  (:`Triggered`
    (`self.SR_SwitchSlot` 0)))

(event `SR_SwitchSlot`
  (params (ActiveSlot :type Integer))
  (if (!= ActiveSlot (`self.ActiveSlot`))
    (`/Engine/EditorBlueprintResources/StandardMacros.DoOnce` false :!label _label
      (:`Completed`
        (set `self.ActiveSlot` ActiveSlot)
        (`KismetSystemLibrary.Delay` 1.0)
        (goto _label :!via `Reset`)))))

(event `self.HealthComponent_BP.OnHealthChange`
  (params (NewHealth :type "Float (double-precision)"))
  ; Health Component
)

(event `Heal Player`
  (params (`Heal Value` :type "Float (double-precision)"))
  (bind _healthcomponent_bp (`self.HealthComponent_BP`))
  ; Healing Player
  (if (and (not (`self.IsDead?`)) (!= (stale `self.HealthComponent_BP.OnHealthChange` NewHealth) (`/Game/HealthAndDamage/HealthComponent_BP.MaxHealth` (`self.HealthComponent_BP`))))
    (set `/Game/HealthAndDamage/HealthComponent_BP.Health` (`KismetMathLibrary.FClamp` (+ `Heal Value` (`/Game/HealthAndDamage/HealthComponent_BP.Health` _healthcomponent_bp)) 0.0 (`/Game/HealthAndDamage/HealthComponent_BP.MaxHealth` _healthcomponent_bp)) _healthcomponent_bp)))

(event `EnhancedInput|/Game/TopDown/Input/Actions/IA_Slot2`
  (params (ActionValue :type Boolean) (ElapsedSeconds :type "Float (double-precision)") (TriggeredSeconds :type "Float (double-precision)") (InputAction :type "InputAction Object Reference" :default "/Game/TopDown/Input/Actions/IA_Slot2.IA_Slot2"))
  (:`Triggered`
    (`self.SR_SwitchSlot` 1)))

(event `SR_DropCurrentWeapon`
  (`self.DropWeapon`))

(event `self.HealthComponent_BP.OnHealthDepletetd`
  ; Health Component
  (`KismetSystemLibrary.PrintString` "Character Die" true true (struct :`R` 0.689583 :`B` 0.046434 :`A` 1.0)))

(event `EnhancedInput|/Game/TopDown/Input/Actions/IA_DropTool`
  (params (ActionValue :type Boolean) (ElapsedSeconds :type "Float (double-precision)") (TriggeredSeconds :type "Float (double-precision)") (InputAction :type "InputAction Object Reference" :default "/Game/TopDown/Input/Actions/IA_DropTool.IA_DropTool"))
  (:`Triggered`
    (`self.SR_DropCurrentWeapon`)))

(event `/Game/TopDown/Blueprints/Interfaces/CharacterStats_BPI.Adjust_Health`
  (params (Adjustment :type "Float (double-precision)")))

(event `EnhancedInput|/Game/TopDown/Input/Actions/IA_Reload`
  (params (ActionValue :type Boolean) (ElapsedSeconds :type "Float (double-precision)") (TriggeredSeconds :type "Float (double-precision)") (InputAction :type "InputAction Object Reference" :default "/Game/TopDown/Input/Actions/IA_Reload.IA_Reload"))
  (bind _childactor (`ChildActorComponent.ChildActor` (`self.ActiveWeapon`)))
  ; Reload
  (:`Triggered`
    (`/Engine/EditorBlueprintResources/StandardMacros.IsValid` _childactor
      (:`Is Valid`
        (message `/Game/Projectile/Inputs_BPI.Input_Reload` _childactor)))))

(fn `DropWeapon`
  (bind _output (`|GetArrayItem` (`self.Inventory`) (`self.ActiveSlot`)))
  (if (not (`KismetStringLibrary.IsEmpty` _output))
    (`|SpawnActorFromClass` "/Game/Projectile/PickUp_Items_BP.PickUp_Items_BP_C" (`KismetMathLibrary.MakeTransform` (`SceneComponent.K2_GetComponentLocation` (`self.ActiveWeapon`))) "AdjustIfPossibleButAlwaysSpawn" "MultiplyWithRoot" null _output null)
    (`KismetArrayLibrary.Array_Set` (`self.Inventory`) (`self.ActiveSlot`))
    (set `self.Inventory` (`self.Inventory`))))

(fn `InteractionTrace`
  (bind _shooting_springarm (`self.Shooting_SpringArm`))
  (bind _returnvalue (`SceneComponent.GetSocketLocation` _shooting_springarm "ActiveWeapon"))
  (if (`self.IsLocallyControlled`)
    (bind _outhit (`KismetSystemLibrary.LineTraceSingle` _returnvalue (+ _returnvalue (* (`SceneComponent.GetForwardVector` _shooting_springarm) (`self.InteractionLength`))) "TraceTypeQuery3"))
    (if true
      (bind (_bblockinghit _binitialoverlap _time _distance _location _impactpoint _normal _impactnormal _physmat _hitactor) (`GameplayStatics.BreakHitResult` _outhit))
      (if (`KismetSystemLibrary.DoesImplementInterface` _hitactor "/Game/TopDown/Blueprints/Interfaces/Interaction_BPI.Interaction_BPI_C")
        (bind _output_get (set `self.InteractionActor` _hitactor))
        (message `/Game/TopDown/Blueprints/Interfaces/Interaction_BPI.SetFocused` _output_get)
        (else
          (`self.InteractionActor`
            (:`then`
              (set `self.InteractionActor` null))
            (:`else`)))))))

(fn `OnRep_ActiveSlot`
  (`self.Update_Tools`))

(fn `OnRep_Health`)

(fn `OnRep_Inventory`
  (`self.Update_Tools`))

(fn `Process_ItemPickup`
  (params (IncomingItemID :type "String (by ref)"))
  (if (`KismetStringLibrary.IsEmpty` (`|GetArrayItem` (`self.Inventory`)))
    (`KismetArrayLibrary.Array_Set` (`self.Inventory`) 0 IncomingItemID)
    (set `self.Inventory` (`self.Inventory`))
    (elif (`KismetStringLibrary.IsEmpty` (`|GetArrayItem` (`self.Inventory`) 1))
      (`KismetArrayLibrary.Array_Set` (`self.Inventory`) 1 IncomingItemID)
      (set `self.Inventory` (`self.Inventory`))
      (else
        (`|SpawnActorFromClass` "/Game/Projectile/PickUp_Items_BP.PickUp_Items_BP_C" (`KismetMathLibrary.MakeTransform` (`SceneComponent.K2_GetComponentLocation` (`self.ActiveWeapon`))) "AdjustIfPossibleButAlwaysSpawn" "MultiplyWithRoot" null (`|GetArrayItem` (`self.Inventory`) (`self.ActiveSlot`)) null)
        (`KismetArrayLibrary.Array_Set` (`self.Inventory`) (`self.ActiveSlot`) IncomingItemID)
        (set `self.Inventory` (`self.Inventory`))))))

(fn `Setup_Tool`)

(fn `ShootProjectile`
  (params (Transform :type "Transform Structure"))
  (bind _weaponchoice (`self.WeaponChoice`))
  (if (== _weaponchoice "Default")
    (`|SpawnActorFromClass` "/Game/Projectile/PlayerProjectile_Default_BP.PlayerProjectile_Default_BP_C" Transform "AdjustIfPossibleButAlwaysSpawn" "MultiplyWithRoot" null null :!label _label)
    (elif (== _weaponchoice "Red")
      (`|SpawnActorFromClass` "/Game/Projectile/PlayerProjectile_ArmorPiercing_BP.PlayerProjectile_ArmorPiercing_BP_C" Transform "AdjustIfPossibleButAlwaysSpawn" "MultiplyWithRoot" null null)
      (else
        (goto _label)))))

(fn `Update_Tools`
  (`|ExecutionSequence`
    (:`then_0`
      (bind _returnvalue (`|GetDataTableRow` "/Game/Data/DT_PickupItems.DT_PickupItems" (`KismetStringLibrary.Conv_StringToName` (`|GetArrayItem` (`self.Inventory`) (`self.ActiveSlot`))))
        (:`then`
          (`ChildActorComponent.SetChildActorClass` (`self.ActiveWeapon`) (`.Blueprint_13_2BFA16A7462033A110A59E92B2F99337` (break `/Game/Data/S_PickupItem` _returnvalue)))
          (`self.Setup_Tool`))
        (:`RowNotFound`
          (`ChildActorComponent.SetChildActorClass` (`self.ActiveWeapon`) null))))
    (:`then_1`
      (for (_array_element _array_index) (`self.Inventory`)
        (if (!= _array_index (`self.ActiveSlot`))
          (bind _returnvalue_2 (`|GetDataTableRow` "/Game/Data/DT_PickupItems.DT_PickupItems" (`KismetStringLibrary.Conv_StringToName` _array_element))
            (:`then`
              (`StaticMeshComponent.SetStaticMesh` (`self.SM_SecondSlot`) (`.SM_Item_7_FF39EB754CED4EF3BD3B679C175FEDCC` (break `/Game/Data/S_PickupItem` _returnvalue_2))))
            (:`RowNotFound`
              (`StaticMeshComponent.SetStaticMesh` (`self.SM_SecondSlot`) null))))))))

(fn `UserConstructionScript`)